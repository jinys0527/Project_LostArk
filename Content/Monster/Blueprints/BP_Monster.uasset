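; BP_Monster is an enemy that deals a very large hit of damage to the top-down player character on contact.
; Its Box component's hit event casts to BP_TopDownCharacter and applies damage only if that character's IsHit flag is clear.
; The monster sets that flag and clears it after a one-second delay as a damage cooldown, printing its value for debugging.
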(event OnComponentHit(Box)
  (params (HitComponent :type Primitive%20Component%20Object%20Reference) (OtherActor :type Actor%20Object%20Reference) (OtherComp :type Primitive%20Component%20Object%20Reference) (NormalImpulse :type Vector :default "0, 0, 0") (Hit :type Hit%20Result%20Structure%20%28by%20ref%29))
  (bind _asbp_top_down_character (Utilities|Casting|CastToBP_TopDownCharacter OtherActor))
  (Development|PrintString (Utilities|String|ToString(Boolean) (Variables|/Game/TopDown/Blueprints/BP_TopDownCharacter.BP_TopDownCharacter_C|GetbIsHit _asbp_top_down_character)))
  (if (not (Variables|/Game/TopDown/Blueprints/BP_TopDownCharacter.BP_TopDownCharacter_C|GetbIsHit _asbp_top_down_character))
    (Variables|/Game/TopDown/Blueprints/BP_TopDownCharacter.BP_TopDownCharacter_C|SetbIsHit _asbp_top_down_character true)
    (Development|PrintString (Utilities|String|ToString(Boolean) (Variables|/Game/TopDown/Blueprints/BP_TopDownCharacter.BP_TopDownCharacter_C|GetbIsHit _asbp_top_down_character)))
    (Game|Damage|ApplyDamage _asbp_top_down_character 123445.0 0 self)
    (Utilities|FlowControl|Delay 1.0)
    (Variables|/Game/TopDown/Blueprints/BP_TopDownCharacter.BP_TopDownCharacter_C|SetbIsHit _asbp_top_down_character false)
    (Development|PrintString (Utilities|String|ToString(Boolean) (Variables|/Game/TopDown/Blueprints/BP_TopDownCharacter.BP_TopDownCharacter_C|GetbIsHit _asbp_top_down_character)))))

(event EventBeginPlay)

(event Collision|EventActorBeginOverlap
  (params (OtherActor :type Actor%20Object%20Reference)))

(event EventTick
  (params (DeltaSeconds :type Float%20%28single-precision%29)))

(fn ConstructionScript)