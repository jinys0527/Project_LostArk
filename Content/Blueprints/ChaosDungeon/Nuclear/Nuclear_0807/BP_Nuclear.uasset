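; BP_Nuclear is a destructible dungeon core that breaks over three hits from the player's equipped greatsword.
; Sword overlaps register the core on the sword, counting as hits only during attacks while the Hitted latch, never reset here, is clear.
; Each hit swaps the visual for a new Geometry Cache stage.
; After the final animation, it calls SpawnSpawner, clears the game mode's IsExistCore flag and destroys itself.
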(event OnComponentBeginOverlap(Nuclear_mesh_collision)
  (params (OverlappedComponent :type Primitive%20Component%20Object%20Reference) (OtherActor :type Actor%20Object%20Reference) (OtherComp :type Primitive%20Component%20Object%20Reference) (OtherBodyIndex :type Integer) (bFromSweep :type Boolean) (SweepResult :type Hit%20Result%20Structure%20%28by%20ref%29))
  (bind _asbp_great_sword (Utilities|Casting|CastToBP_GreatSword OtherActor))
  (Variables|/Script/LostArk.GreatSword|SetOverlappedCore _asbp_great_sword self)
  (bind _asbp_chaos_dungeon_player (Utilities|Casting|CastToBP_ChaosDungeonPlayer (Game|Player|GetPlayerPawn 0)))
  (if (== _asbp_great_sword (Variables|/Script/LostArk.MyPlayer|GetEquippedGreatSword _asbp_chaos_dungeon_player))
    (if (and (Variables|/Script/LostArk.MyPlayer|GetbIsAttack _asbp_chaos_dungeon_player) (not (Variables|Default|GetHitted)))
      (Variables|Default|SetHitted true)
      (bind _output_get (Variables|Default|SetHit (+ (Variables|Default|GetHit) 1)))
      (switch int _output_get
        (:1
          (Rendering|SetVisibility (Variables|Default|GetNuclear_mesh_collision) false false)
          (bind _returnvalue (AddComponent|AddGeometryCacheComponent false)))
        (:2
          (Rendering|SetVisibility _returnvalue false false)
          (bind _returnvalue_2 (AddComponent|AddGeometryCacheComponent false))
          (Components|DestroyComponent _returnvalue))
        (:3
          (Rendering|SetVisibility _returnvalue_2 false false)
          (bind _returnvalue_3 (AddComponent|AddGeometryCacheComponent false))
          (Components|DestroyComponent _returnvalue_2)
          (Collision|SetCollisionEnabled (Variables|Default|GetNuclear_mesh_collision) "NoCollision")
          (Utilities|FlowControl|Delay (Media|MediaPlayer|GetDuration _returnvalue_3))
          (Components|DestroyComponent _returnvalue_3)
          (Class|ChaosDungeonCore|SpawnSpawner)
          (bind _aschaos_dungeon_mode (Utilities|Casting|CastToChaosDungeonMode (Game|GetGameMode)))
          (Variables|/Script/LostArk.ChaosDungeonMode|SetbIsExistCore _aschaos_dungeon_mode false)
          (Actor|DestroyActor))))))

(fn ConstructionScript)