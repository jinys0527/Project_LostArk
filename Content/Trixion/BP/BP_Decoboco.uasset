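; BP_Decoboco is an animated Blueprint with four static meshes that pivot in opposing pairs.
; On BeginPlay it plays a timeline whose RotationTimeline track interpolates pitch between zero and the Rot variable.
; StaticMesh3 and StaticMesh1 pitch toward Rot, while StaticMesh2 and StaticMesh pitch toward its negative, with roll and yaw held at zero.
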(event EventBeginPlay
  (bind _rot (Variables|Default|GetRot))
  (bind _rotationtimeline (Timeline|Timeline Play)
    (:Update
      (Utilities|FlowControl|Sequence
        (:then_0
          (Transformation|SetRelativeRotation (Variables|Default|GetStaticMesh3) (Math|Rotator|MakeRotator 0.0 (Math|Float|Lerp 0.0 _rot _rotationtimeline) 0.0) false false))
        (:then_1
          (Transformation|SetRelativeRotation (Variables|Default|GetStaticMesh2) (Math|Rotator|MakeRotator 0.0 (Math|Float|Lerp 0.0 (* _rot -1.0) _rotationtimeline) 0.0) false false))))))

(fn ConstructionScript)